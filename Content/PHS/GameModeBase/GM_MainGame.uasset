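; GM_MainGame is the game mode for the main game and handles spawning player characters.
; On PostLogin, it passes the new player controller to the RespawnPlayer event.
; RespawnPlayer spawns a BP_MainCharacter at a randomly chosen PlayerStart and has the controller possess it.
; It does not destroy any previous pawn or check whether the chosen start is occupied.
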(event `RespawnPlayer`
  (params (PC :type "PlayerController Object Reference"))
  ;[1 1 1] 코멘트
  (`/Engine/EditorBlueprintResources/StandardMacros.IsValid` PC
    (:`Is Valid`
      (bind _outactors (`GameplayStatics.GetAllActorsOfClass` "/Script/Engine.PlayerStart"))
      (bind _returnvalue (`|SpawnActorFromClass` "/Game/PHS/Character/BP_MainCharacter.BP_MainCharacter_C" (`self.GetTransform` (`|GetArrayItem` _outactors (`KismetMathLibrary.RandomIntegerInRange` 0 (- (`KismetArrayLibrary.Array_Length` _outactors) 1)))) "Undefined" "OverrideRootScale" null null))
      (`Controller.Possess` PC _returnvalue))))

(event `self.K2_PostLogin`
  (params (NewPlayer :type "PlayerController Object Reference"))
  ;[1 1 1] 코멘트
  (`self.RespawnPlayer` NewPlayer))

(fn `UserConstructionScript`)