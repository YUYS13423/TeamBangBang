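; BP_Sniper is a sniper weapon actor, largely unfinished: most weapon functions are stubs, and its hand-attach and overlay-creation setup is unwired.
; ZoonIn calls SniperZoom, which toggles aiming and the scope overlay, blending the view to the sniper on both toggles.
; FireFX spawns separate owner-only and owner-hidden muzzle flashes on the authority, plus conditional impact particles.
; Stop_FX destroys valid actors, with an explosion emitter.
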(event `OnWeaponFIre`)

(event `OffWeaponFire`
  (`|ExecutionSequence`))

(event `self.ReceiveBeginPlay`
  (`self.Sniper Set`))

(event `Start_FX`)

(event `Stop_FX`
  (`|ExecutionSequence`
    (:`then_0`
      (`/Engine/EditorBlueprintResources/StandardMacros.IsValid` null
        (:`Is Valid`
          (`self.K2_DestroyActor`)
          (`GameplayStatics.SpawnEmitterAttached` "/Game/StarterContent/Particles/P_Explosion.P_Explosion"))))
    (:`then_1`
      (`/Engine/EditorBlueprintResources/StandardMacros.IsValid` null
        (:`Is Valid`
          (`self.K2_DestroyActor`))))))

(fn `Drop`
  (returns (NewParam :type Boolean))
  (return false))

(fn `FireFX`
  (params (Condition :type Boolean) (Hit :type "HitResult Structure (by ref)"))
  (bind (_bblockinghit _binitialoverlap _time _distance _location _impactpoint _normal _impactnormal) (`GameplayStatics.BreakHitResult` Hit))
  (bind _returnvalue (`KismetMathLibrary.MakeTransform` (0.0 0.0 0.0)))
  (bind _returnvalue_2 (`self.GetOwner`))
  (`|ExecutionSequence`
    (:`then_0`
      (`/Engine/EditorBlueprintResources/ActorMacros.Switch Has Authority`
        (:`Authority`
          (`|ExecutionSequence`
            (:`then_0`
              (`/Engine/EditorBlueprintResources/StandardMacros.IsValid` (`self.F_Flash`)
                (:`Is Not Valid`
                  (bind _returnvalue_3 (`|SpawnActorFromClass` "/Game/PHS/Weapon/BP_FxFire.BP_FxFire_C" _returnvalue "AlwaysSpawn" "OverrideRootScale" _returnvalue_2 null))
                  (bind _output_get (set `self.F_Flash` _returnvalue_3))
                  (`self.K2_AttachToComponent` _output_get null "Muzzle" "SnapToTarget" "SnapToTarget" "KeepRelative" true)
                  (`/Game/PHS/Weapon/BP_FxFire.SetOwnerSee` _output_get))))
            (:`then_1`
              (`/Engine/EditorBlueprintResources/StandardMacros.IsValid` (`self.M_Flash`)
                (:`Is Not Valid`
                  (bind _returnvalue_4 (`|SpawnActorFromClass` "/Game/PHS/Weapon/BP_FxFire.BP_FxFire_C" _returnvalue "AlwaysSpawn" "OverrideRootScale" _returnvalue_2 null))
                  (bind _output_get_2 (set `self.M_Flash` _returnvalue_4))
                  (`self.K2_AttachToComponent` _output_get_2 null "Muzzle" "SnapToTarget" "SnapToTarget" "KeepRelative" true)
                  (`/Game/PHS/Weapon/BP_FxFire.SetOwnerNoSee` _output_get_2))))))))
    (:`then_1`
      (if Condition
        (`GameplayStatics.SpawnEmitterAtLocation` null _impactpoint (`KismetMathLibrary.MakeRotFromZ` _impactnormal))))))

(fn `Firing`
  (returns (NewParam :type Boolean))
  (return false))

(fn `Get`
  (returns (NewParam :type Boolean))
  (return false))

(fn `Reload`
  (returns (NewParam :type Boolean))
  (return false))

(fn `RemainedAmmo`
  (returns (NewParam :type Boolean))
  (`KismetSystemLibrary.PrintString` "Hello")
  (return true))

(fn `Select`
  (returns (NewParam :type Boolean))
  (return false))

(fn `Sniper Set`)

(fn `SniperZoom`
  (bind _returnvalue (`GameplayStatics.GetPlayerController` 0))
  (bind _overlayref (`self.OverlayREF`))
  (`/Engine/EditorBlueprintResources/StandardMacros.FlipFlop`
    (:`A`
      (set `self.IsAiming?` true)
      (`PlayerController.SetViewTargetWithBlend` _returnvalue self 0.2 "VTBlend_Linear" 0.0 false)
      (`UserWidget.AddToViewport` _overlayref 0))
    (:`B`
      (set `self.IsAiming?` false)
      (`PlayerController.SetViewTargetWithBlend` _returnvalue self 0.2 "VTBlend_Linear" 0.0 false)
      (`Widget.RemoveFromParent` _overlayref))))

(fn `UserConstructionScript`)

(fn `ZoonIn`
  (returns (NewParam :type Boolean))
  (`self.SniperZoom`)
  (return false))