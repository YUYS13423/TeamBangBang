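; Master weapon Blueprint that handles single and automatic fire, clip and reserve ammo, reloading, and shot effects.
; Firing runs a randomly spread camera trace, then retraces from the first-person muzzle to that point for damage and impacts.
; Auto fire loops through a gated delay macro.
; The authority initializes and refills ammo and spawns separate muzzle flashes with owner-see and owner-no-see visibility.
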(event `ReloadFX`
  ;[1 1 1] Sound:Reload, Delay
  (`GameplayStatics.SpawnSound2D` null 1.0 1.0 0.0 null))

(event `OnReloadWeapon`
  ;[1 1 1] Sound:Reload, Delay
  (`self.ReloadFX`)
  (`KismetSystemLibrary.Delay` 2.0)
  (`self.ReloadAddAmmo`))

(event `self.ReceiveBeginPlay`
  ;[1 1 1] Server : Current Ammo, Clip Size Set
  (`/Engine/EditorBlueprintResources/ActorMacros.Switch Has Authority`
    (:`Authority`
      (set `self.CurrentMaxAmmo` (`self.MaxAmmo`))
      (set `self.CurrentAmmoInclip` (`self.MaxAmmoClipSize`)))))

(event `Start_FX`
  (params (Condition :type Boolean) (Hit :type "HitResult Structure (by ref)"))
  ;[1 1 1] Fire : Start, Stop
  (`self.FireFX` Condition Hit)
  (switch `/Game/PHS/Weapon/FireMode` (`self.E_fireMode`)
    (:`NewEnumerator0`
      (`KismetSystemLibrary.Delay` 0.17)
      (`self.Stop_FX`))))

(event `Stop_FX`
  (bind _m_flash (`self.M_Flash`))
  (bind _f_flash (`self.F_Flash`))
  ;[1 1 1] Fire : Start, Stop
  (`|ExecutionSequence`
    (:`then_0`
      (`/Engine/EditorBlueprintResources/StandardMacros.IsValid` _f_flash
        (:`Is Valid`
          (`self.K2_DestroyActor` _f_flash))))
    (:`then_1`
      (`/Engine/EditorBlueprintResources/StandardMacros.IsValid` _m_flash
        (:`Is Valid`
          (`self.K2_DestroyActor` _m_flash))))))

(event `Shootinf`
  (params (Hit :type "HitResult Structure (by ref)") (IsHit :type Boolean) (FMzzle :type "Vector Structure") (MMzzle :type "Vector Structure"))
  ;[1 1 1] 코멘트
  (bind _output_get (set `self.CurrentAmmoInclip` (`KismetMathLibrary.Clamp` (- (`self.CurrentAmmoInclip`) 1) 0 (`self.MaxAmmoClipSize`))))
  (if (not (== _output_get 0))
    (`self.Start_FX` IsHit Hit)
    (if IsHit
      (`GameplayStatics.ApplyDamage` (`.HitActor` (`GameplayStatics.BreakHitResult` Hit)) 10.0 (`self.GetInstigatorController`) self))
    (else
      (`/Game/PHS/Character/BP_MainCharacter.StopWeaponFire` (`self.BP_MainCharacter`)))))

(event `OnWeaponFire`
  ;[1 1 1] 코멘트
  (switch `/Game/PHS/Weapon/FireMode` (`self.E_fireMode`)
    (:`NewEnumerator0`
      _)
    (:`NewEnumerator1`
      (`self.AutoFireMode` :!label _label
        (:`then_0`
          _))))
  (bind (_outhit _returnvalue _returnvalue1 _returnvalue2) (`self.SphereTrace`))
  (`self.Shootinf` _outhit _returnvalue _returnvalue1 _returnvalue2))

(event `OffWeaponFire`
  ;[1 1 1] 코멘트
  (`|ExecutionSequence`
    (:`then_0`
      (goto _label :!via `Close`))
    (:`then_1`
      (`self.Stop_FX`))))

(fn `FireFX`
  (params (Condition :type Boolean) (Hit :type "HitResult Structure (by ref)"))
  (bind _returnvalue (`self.GetOwner`))
  (bind _returnvalue_2 (`KismetMathLibrary.MakeTransform` (0.0 0.0 0.0)))
  (bind (_bblockinghit _binitialoverlap _time _distance _location _impactpoint _normal _impactnormal) (`GameplayStatics.BreakHitResult` Hit))
  (`|ExecutionSequence`
    (:`then_0`
      (`/Engine/EditorBlueprintResources/ActorMacros.Switch Has Authority`
        (:`Authority`
          (`|ExecutionSequence`
            (:`then_0`
              (`/Engine/EditorBlueprintResources/StandardMacros.IsValid` (`self.F_Flash`)
                (:`Is Not Valid`
                  (bind _returnvalue_3 (`|SpawnActorFromClass` "/Game/PHS/Weapon/BP_FxFire.BP_FxFire_C" _returnvalue_2 "AlwaysSpawn" "OverrideRootScale" _returnvalue null))
                  (bind _output_get (set `self.F_Flash` _returnvalue_3))
                  (`self.K2_AttachToComponent` _output_get null "Muzzle" "SnapToTarget" "SnapToTarget" "KeepRelative" true)
                  (`/Game/PHS/Weapon/BP_FxFire.SetOwnerSee` _output_get))))
            (:`then_1`
              (`/Engine/EditorBlueprintResources/StandardMacros.IsValid` (`self.M_Flash`)
                (:`Is Not Valid`
                  (bind _returnvalue_4 (`|SpawnActorFromClass` "/Game/PHS/Weapon/BP_FxFire.BP_FxFire_C" _returnvalue_2 "AlwaysSpawn" "OverrideRootScale" _returnvalue null))
                  (bind _output_get_2 (set `self.M_Flash` _returnvalue_4))
                  (`self.K2_AttachToComponent` _output_get_2 null "Muzzle" "SnapToTarget" "SnapToTarget" "KeepRelative" true)
                  (`/Game/PHS/Weapon/BP_FxFire.SetOwnerNoSee` _output_get_2))))))))
    (:`then_1`
      (if Condition
        (`GameplayStatics.SpawnEmitterAtLocation` null _impactpoint (`KismetMathLibrary.MakeRotFromZ` _impactnormal))))))

(fn `ReloadAddAmmo`
  (`/Engine/EditorBlueprintResources/ActorMacros.Switch Has Authority`
    (:`Authority`
      (bind _output_get (set `self.AmmoNeedForReload` (- (`self.MaxAmmoClipSize`) (`self.CurrentAmmoInclip`))))
      (if (<= (`self.CurrentMaxAmmo`) _output_get)
        (set `self.CurrentAmmoInclip` (+ (`self.CurrentAmmoInclip`) (`self.CurrentMaxAmmo`)))
        (set `self.CurrentMaxAmmo` 0)
        (else
          (set `self.CurrentMaxAmmo` (- (`self.CurrentMaxAmmo`) (`self.AmmoNeedForReload`)))
          (set `self.CurrentAmmoInclip` (`self.MaxAmmoClipSize`)))))))

(fn `SphereTrace`
  (returns (OutHit :type "HitResult Structure") (ReturnValue :type Boolean) (ReturnValue1 :type "Vector Structure") (ReturnValue2 :type "Vector Structure"))
  (bind _returnvalue (`GameplayStatics.GetPlayerCameraManager` 0))
  (bind _returnvalue_2 (`SceneComponent.GetSocketLocation` (`self.SK_F_Mesh`) "Muzzle"))
  (bind _returnvalue_3 (`PlayerCameraManager.GetCameraLocation` _returnvalue))
  (bind (_outhit _returnvalue_4) (`KismetSystemLibrary.SphereTraceSingle` _returnvalue_3 (+ (+ _returnvalue_3 (* (`KismetMathLibrary.GetForwardVector` (`PlayerCameraManager.GetCameraRotation` _returnvalue)) 5000.0)) (* (`KismetMathLibrary.RandomUnitVector`) (`KismetMathLibrary.RandomFloatInRange` 0.0 300.0))) 0.0 "TraceTypeQuery1" false (`|MakeArray` (`self.GetOwner`))))
  (bind (_bblockinghit _binitialoverlap _time _distance _location _impactpoint _normal _impactnormal _physmat _hitactor _hitcomponent _hitbonename _hititem _elementindex _faceindex _tracestart _traceend) (`GameplayStatics.BreakHitResult` _outhit))
  (bind (_outhit_2 _returnvalue_5) (`KismetSystemLibrary.SphereTraceSingle` _returnvalue_2 (select `bool` _returnvalue_4 :`false` _traceend :`true` _impactpoint) 0.0 "TraceTypeQuery1"))
  (return _outhit_2 _returnvalue_5 _returnvalue_2 (`SceneComponent.GetSocketLocation` (`self.SK_M_Mesh`) "Muzzle")))

(fn `UserConstructionScript`)