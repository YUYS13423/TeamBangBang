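; Thrown smoke grenade projectile that flies from its owner and destroys itself 20 seconds after spawning.
; The construction script launches ProjectileMovement with VelocityX and VelocityZ plus most of the CharacterTest owner's velocity.
; Tick uses a signed velocity check to detect slowing, then once makes the shell mesh ignore Pawn collision.
; Weapon functions are false-returning stubs, and the three-second delay triggers nothing.
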(event `self.ReceiveBeginPlay`
  (`|ExecutionSequence`
    (:`then_0`
      (`KismetSystemLibrary.Delay` 3.0))
    (:`then_1`
      (`KismetSystemLibrary.Delay` 20.0)
      (`self.K2_DestroyActor`))))

(event `self.ReceiveTick`
  (params (DeltaSeconds :type "Float (single-precision)"))
  (bind (_returnvalue_x _returnvalue_y _returnvalue_z) (`KismetMathLibrary.BreakVector` (`self.GetVelocity`)))
  (if (and (< (+ _returnvalue_x _returnvalue_y) 100.0) (< _returnvalue_z 10.0))
    (`/Engine/EditorBlueprintResources/StandardMacros.IsValid` self
      (:`Is Valid`
        (`/Engine/EditorBlueprintResources/StandardMacros.DoOnce` false
          (:`Completed`
            (`SceneComponent.K2_SetWorldLocation` (`self.SM_SmokeShell`) (`SceneComponent.K2_GetComponentLocation` (`self.SM_SmokeShell`)) false false)
            (`PrimitiveComponent.SetCollisionResponseToChannel` (`self.SM_SmokeShell`) "ECC_Pawn" "ECR_Ignore")))))))

(fn `Drop`
  (returns (NewParam :type Boolean))
  (return false))

(fn `Firing`
  (returns (NewParam :type Boolean))
  (return false))

(fn `Get`
  (returns (NewParam :type Boolean))
  (return false))

(fn `Reload`
  (returns (NewParam :type Boolean))
  (return false))

(fn `RemainedAmmo`
  (returns (NewParam :type Boolean))
  (return false))

(fn `Select`
  (returns (NewParam :type Boolean))
  (return false))

(fn `UserConstructionScript`
  (bind _returnvalue (`self.GetOwner`))
  (`/Engine/EditorBlueprintResources/StandardMacros.IsValid` _returnvalue
    (:`Is Valid`
      (cast `/Game/YYS/Character/CharacterTest` _returnvalue)
      (set `self.Ownerisme` (`self.Ownerisme`))
      (bind _output_get (set `MovementComponent.Velocity` (`KismetMathLibrary.MakeVector` (+ (`self.Velocity X`) (.x (* (`self.GetVelocity` (`self.Ownerisme`)) 0.8))) (.y (* (`self.GetVelocity` (`self.Ownerisme`)) 0.8)) (+ (.z (* (`self.GetVelocity` (`self.Ownerisme`)) 0.8)) (`self.Velocity Z`))) (`self.ProjectileMovement`)))
      (set `ProjectileMovementComponent.InitialSpeed` (`KismetMathLibrary.VSize` _output_get) (`self.ProjectileMovement`)))))

(fn `ZoonIn`
  (returns (NewParam :type Boolean))
  (return false))