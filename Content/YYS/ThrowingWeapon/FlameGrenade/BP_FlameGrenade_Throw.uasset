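; Thrown flame grenade projectile that leaves a Fire actor where it lands and destroys itself.
; The construction script sets launch velocity from VelocityX/VelocityZ plus 80% of the owning CharacterTest's velocity.
; On mesh hit, a short downward trace must find a surface before Fire spawns; otherwise a timed self-destruct cleans up.
; Debug trace drawing and per-tick speed printing remain; weapon functions like Firing and Reload are false-returning stubs.
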(event `self.ReceiveBeginPlay`
  (`KismetSystemLibrary.Delay` 4.0)
  (`/Engine/EditorBlueprintResources/StandardMacros.IsValid` self
    (:`Is Valid`
      (`self.K2_DestroyActor`))))

(event `self.SM_FlameGrenade.OnComponentHit`
  (params (HitComponent :type "PrimitiveComponent Object Reference") (OtherActor :type "Actor Object Reference") (OtherComp :type "PrimitiveComponent Object Reference") (NormalImpulse :type "Vector Structure") (Hit :type "HitResult Structure (by ref)"))
  (bind _scene (`self.Scene`))
  (bind _returnvalue (`SceneComponent.K2_GetComponentLocation` _scene))
  (bind (_returnvalue_roll _returnvalue_pitch _returnvalue_yaw) (`KismetMathLibrary.BreakRotator` (`SceneComponent.K2_GetComponentRotation` _scene)))
  (bind (_outhit _returnvalue_2) (`KismetSystemLibrary.LineTraceSingle` :`Start` _returnvalue :`End` (- _returnvalue (0.0 0.0 18.0)) :`TraceChannel` "TraceTypeQuery1" :`DrawDebugType` "ForDuration" :`TraceColor` (struct :`R` 0.025236 :`B` 1.0 :`A` 1.0) :`DrawTime` 20.0))
  (if _returnvalue_2
    (`|SpawnActorFromClass` "/Game/YYS/ThrowingWeapon/FlameGrenade/Fire.Fire_C" (`KismetMathLibrary.MakeTransform` (`.ImpactPoint` (`GameplayStatics.BreakHitResult` _outhit)) (`KismetMathLibrary.MakeRotator` 0.0 0.0 _returnvalue_yaw)) "Undefined" "OverrideRootScale" null null)
    (`self.K2_DestroyActor`)))

(event `self.ReceiveTick`
  (params (DeltaSeconds :type "Float (single-precision)"))
  (`KismetSystemLibrary.PrintString` (`KismetStringLibrary.Conv_DoubleToString` (`KismetMathLibrary.VSize` (`self.GetVelocity`))) true true (struct :`G` 0.66 :`B` 1.0 :`A` 1.0) 0.0))

(fn `Drop`
  (returns (NewParam :type Boolean))
  (return false))

(fn `Firing`
  (returns (NewParam :type Boolean))
  (return false))

(fn `Get`
  (returns (NewParam :type Boolean))
  (return false))

(fn `Reload`
  (returns (NewParam :type Boolean))
  (return false))

(fn `RemainedAmmo`
  (returns (NewParam :type Boolean))
  (return false))

(fn `Select`
  (returns (NewParam :type Boolean))
  (return false))

(fn `UserConstructionScript`
  (bind _returnvalue (`self.GetOwner`))
  (`/Engine/EditorBlueprintResources/StandardMacros.IsValid` _returnvalue
    (:`Is Valid`
      (bind _ascharacter_test (cast `/Game/YYS/Character/CharacterTest` _returnvalue))
      (set `self.Ownerisme` _ascharacter_test)
      (bind _output_get (set `MovementComponent.Velocity` (`KismetMathLibrary.MakeVector` (+ (`self.Velocity X`) (.x (* (`self.GetVelocity` (`self.Ownerisme`)) 0.8))) (.y (* (`self.GetVelocity` (`self.Ownerisme`)) 0.8)) (+ (.z (* (`self.GetVelocity` (`self.Ownerisme`)) 0.8)) (`self.Velocity Z`))) (`self.ProjectileMovement`)))
      (set `ProjectileMovementComponent.InitialSpeed` (`KismetMathLibrary.VSize` _output_get) (`self.ProjectileMovement`)))))

(fn `ZoonIn`
  (returns (NewParam :type Boolean))
  (return false))